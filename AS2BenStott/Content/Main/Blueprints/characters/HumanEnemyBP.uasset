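; HumanEnemyBP is a human enemy that takes damage and reacts to seeing the player character.
; AnyDamage subtracts from Health, clamped between zero and MaxHealth.
; Pawn sensing passes seen pawns to EnemyAttack, which casts to characterBP and rotates the enemy to face it.
; The attack checks CanAttack, Isdead and PlayerDead but performs no action afterward, and nothing here sets the death state.
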(event OnSeePawn(PawnSensing)
  (params (Pawn :type Pawn%20Object%20Reference))
  (CallFunction|EnemyAttack Pawn))

(event Game|Damage|EventAnyDamage
  (params (Damage :type Float%20%28single-precision%29) (DamageType :type Damage%20Type%20Object%20Reference) (InstigatedBy :type Controller%20Object%20Reference) (DamageCauser :type Actor%20Object%20Reference))
  (Variables|Default|Sethealth (Math|Float|Clamp(Float) (- (Variables|Default|Gethealth) Damage) 0.0 (Variables|Default|GetmaxHealth))))

(fn ConstructionScript)

(fn EnemyAttack
  (params (Object :type Object%20Object%20Reference))
  (bind _ascharacter_bp (Utilities|Casting|CastTocharacterBP Object))
  (Transformation|SetActorRotation (Math|Rotator|FindRelativeLookatRotation (Math|Conversions|ToTransform(Vector) (Transformation|GetActorLocation)) (Transformation|GetActorLocation _ascharacter_bp)))
  (if (Variables|Default|GetcanAttack)
    (if (not (Variables|Default|Getisdead))
      (if (not (Variables|/Game/Main/Blueprints/characters/characterBP.characterBP_C|GetplayerDead _ascharacter_bp))
        _))))