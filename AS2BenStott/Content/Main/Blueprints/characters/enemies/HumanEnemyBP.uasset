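; HumanEnemyBP is a human enemy that shoots at the player with a pistol.
; When PawnSensing sees a characterBP, it turns to face it and, if attack and alive checks pass, waits on a one-second Delay.
; It then spawns a BallOfDoomBP projectile with muzzle explosion effect and gunshot sound.
; Damage lowers clamped Health, but no death logic appears here, and EnemyAttack is an empty stub.
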(event OnSeePawn(PawnSensing)
  (params (Pawn :type Pawn%20Object%20Reference))
  (bind _pistol (Variables|Default|Getpistol))
  (bind _returnvalue (Transformation|GetSocketLocation _pistol "muzzle"))
  (bind _ascharacter_bp (Utilities|Casting|CastTocharacterBP Pawn))
  (Transformation|SetActorRotation (Math|Rotator|FindRelativeLookatRotation (Math|Conversions|ToTransform(Vector) (Transformation|GetActorLocation)) (Transformation|GetActorLocation _ascharacter_bp)))
  (if (Variables|Default|GetcanAttack)
    (if (not (Variables|Default|Getisdead))
      (if (not (Variables|/Game/Main/Blueprints/characters/characterBP.characterBP_C|GetplayerDead _ascharacter_bp))
        (Utilities|FlowControl|Delay 1.0)
        (Game|SpawnActorfromClass "/Game/Main/Blueprints/weapon/BallOfDoomBP.BallOfDoomBP_C" (Transformation|GetWorldTransform (Variables|Default|GetprojectileSpawn)) "Undefined" "MultiplyWithRoot" 0 0)
        (Effects|SpawnEmitteratLocation "/Game/StarterContent/Particles/P_Explosion.P_Explosion" _returnvalue "0, 0, 0" "0.300000,0.300000,0.300000")
        (Audio|PlaySoundatLocation "/Game/Main/Imported/sounds/makarov-shoot-36241.makarov-shoot-36241" _returnvalue "0, 0, 0" 1.0 1.0 0.0 0 0 0 0)))))

(event Game|Damage|EventAnyDamage
  (params (Damage :type Float%20%28single-precision%29) (DamageType :type Damage%20Type%20Object%20Reference) (InstigatedBy :type Controller%20Object%20Reference) (DamageCauser :type Actor%20Object%20Reference))
  (Variables|Default|Sethealth (Math|Float|Clamp(Float) (- (Variables|Default|Gethealth) Damage) 0.0 (Variables|Default|GetmaxHealth))))

(fn ConstructionScript)

(fn EnemyAttack
  (params (Object :type Object%20Object%20Reference)))