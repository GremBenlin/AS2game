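; Enemy turret actor that shoots at the player character on sight and destroys itself when its health runs out.
; PawnSensing snaps its rotation toward the seen characterBP and, if attacking is allowed and the player is alive, fires a short-delayed line trace from the pistol muzzle to apply damage.
; When player health reaches zero, it disables the player's input and movement, ragdolls the mesh and pushes it with an impulse opposite the hit normal.
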(event OnSeePawn(PawnSensing)
  (params (Pawn :type Pawn%20Object%20Reference))
  (bind _pistol (Variables|Default|Getpistol))
  (bind _base_damage (Variables|Default|GetBase%20Damage))
  (bind _returnvalue (Transformation|GetSocketLocation _pistol "muzzle"))
  (bind _ascharacter_bp (Utilities|Casting|CastTocharacterBP Pawn))
  (Transformation|SetActorRotation (Math|Rotator|FindRelativeLookatRotation (Math|Conversions|ToTransform(Vector) (Transformation|GetActorLocation)) (Transformation|GetActorLocation _ascharacter_bp)))
  (if (Variables|Default|GetcanAttack)
    (if (not (Variables|/Game/Main/Blueprints/characters/characterBP.characterBP_C|GetplayerDead _ascharacter_bp))
      (Utilities|FlowControl|Delay 0.1)
      (bind _outhit (Collision|LineTraceByChannel _returnvalue (+ _returnvalue (* (Math|Vector|GetForwardVector (Transformation|GetActorRotation)) (Variables|Default|Getrange))) "TraceTypeQuery1" false 0 "ForDuration"))
      (Variables|Default|Setimpact%20origin (.Normal (Collision|BreakHitResult _outhit)))
      (Game|Damage|ApplyDamage (.HitActor (Collision|BreakHitResult _outhit)) (Variables|Default|GetBase%20Damage) 0 0)
      (if (<= (Variables|/Game/Main/Blueprints/characters/characterBP.characterBP_C|GetplayerHealth _ascharacter_bp) 0.0)
        (Physics|SetSimulatePhysics (Variables|/Script/Engine.Character|GetMesh _ascharacter_bp) true)
        (Collision|SetCollisionProfileName (Variables|/Script/Engine.Character|GetMesh _ascharacter_bp) "RagDoll" true :!class /Script/Engine.PrimitiveComponent)
        (Pawn|Components|CharacterMovement|DisableMovement (Variables|/Script/Engine.Character|GetCharacterMovement _ascharacter_bp))
        (Input|DisableInput _ascharacter_bp (Game|GetPlayerController 0))
        (Physics|AddImpulseatLocation (Variables|/Script/Engine.Character|GetMesh _ascharacter_bp) (Math|Vector|MakeVector (* _base_damage (* (.x (Variables|Default|Getimpact%20origin)) -1e+01)) (* _base_damage (* (.y (Variables|Default|Getimpact%20origin)) -1e+01)) (* _base_damage (* (.z (Variables|Default|Getimpact%20origin)) -1e+01))) (.ImpactPoint (Collision|BreakHitResult _outhit)) "None")))))

(event Game|Damage|EventAnyDamage
  (params (Damage :type Float%20%28single-precision%29) (DamageType :type Damage%20Type%20Object%20Reference) (InstigatedBy :type Controller%20Object%20Reference) (DamageCauser :type Actor%20Object%20Reference))
  (bind _output_get (Variables|Default|Sethealth (Math|Float|Clamp(Float) (- (Variables|Default|Gethealth) Damage) 0.0 (Variables|Default|GetmaxHealth))))
  (Development|PrintString (Utilities|String|ToString(Float) _output_get))
  (if (<= (Variables|Default|Gethealth) 0.0)
    (Actor|DestroyActor)))

(fn ConstructionScript)