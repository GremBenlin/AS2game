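; Player character Blueprint with Enhanced Input movement, mouse-cursor aiming and a debug-drawn pistol trace.
; BeginPlay adds the default mapping context and shows the cursor; movement follows control-rotation yaw.
; Tick turns only actor yaw toward the visibility hit under the cursor, using constant-speed interpolation.
; Shooting traces from the pistol's muzzle socket along actor forward for a set range, without yet using the hit.
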(event Input|EnhancedActionEvents|EnhancedInputActionIA_movement
  (params (ActionValue :type Vector%202D%20Structure) (ElapsedSeconds :type Float%20%28double-precision%29) (TriggeredSeconds :type Float%20%28double-precision%29) (InputAction :type Input%20Action%20Object%20Reference :default "/Game/Main/Input/Actions/IA_movement.IA_movement"))
  (bind _returnvalue (Pawn|GetControlRotation :!class /Script/Engine.Pawn))
  (bind _returnvalue_2 (Pawn|GetControlRotation :!class /Script/Engine.Pawn))
  (:Triggered
    ;[1 1 1] left/right movement
    (Pawn|Input|AddMovementInput (Math|Vector|GetRightVector (Math|Rotator|MakeRotator (.roll _returnvalue) 0.0 (.yaw _returnvalue))) (.x ActionValue) false)
    ;[1 1 1] forward/backward movement
    (Pawn|Input|AddMovementInput (Math|Vector|GetForwardVector (Math|Rotator|MakeRotator (.roll _returnvalue_2) 0.0 (.yaw _returnvalue_2))) (.y ActionValue) false)))

(event EventTick
  (params (DeltaSeconds :type Float%20%28single-precision%29))
  (bind _returnvalue (Transformation|GetActorRotation))
  ;[1 1 1] sets the character rotation to where the curser is
  (Transformation|SetActorRotation (Math|Rotator|MakeRotator (.roll _returnvalue) (.pitch _returnvalue) (.yaw (Class|KismetMathLibrary|RInterptoConstant (Transformation|GetActorRotation) (Math|Rotator|FindLookatRotation (+ "" "") (- (.ImpactPoint (Collision|BreakHitResult (.HitResult (Game|Player|GetHitResultUnderCursorbyChannel (Game|GetPlayerController 0) "TraceTypeQuery1" true)))) (Transformation|GetActorLocation))) (Utilities|Time|GetWorldDeltaSeconds) (Variables|Default|GetrotationSpeed))))))

(event EventBeginPlay
  ;[1 1 1] gets controller mapping and checks if it's true
  (bind _asplayer_controller (Utilities|Casting|CastToPlayerController (Pawn|GetController)))
  (Utilities|IsValid (PlayerController|LocalPlayerSubsystems|GetEnhancedInputLocalPlayerSubsystem _asplayer_controller)
    (:Is%20Valid
      (Input|AddMappingContext (PlayerController|LocalPlayerSubsystems|GetEnhancedInputLocalPlayerSubsystem _asplayer_controller) "/Game/Main/Input/IMC_Default.IMC_Default" 0 "(bIgnoreAllPressedKeysUntilRelease=True,bForceImmediately=False)")
      ;[1 0 0] curser W.I.P
      (Variables|/Script/Engine.PlayerController|SetbShowMouseCursor (Game|GetPlayerController 0) true))))

(event Input|ActionEvents|InputActionshootAction
  (params (Key :type Key%20Structure))
  (bind _pistol (Variables|Default|Getpistol))
  (bind _returnvalue (Transformation|GetSocketLocation _pistol "muzzle"))
  ;[1 1 1] line trace going from the muzzle going forward from character rotation
  (:Pressed
    (Collision|LineTraceByChannel _returnvalue (+ _returnvalue (* (Math|Vector|GetForwardVector (Transformation|GetActorRotation)) (Variables|Default|Getrange))) "TraceTypeQuery1" false 0 "ForDuration")))

(fn ConstructionScript)