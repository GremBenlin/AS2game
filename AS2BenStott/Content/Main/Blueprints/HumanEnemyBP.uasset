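; HumanEnemyBP is a human enemy that tracks health and has a ragdoll death routine.
; Radial damage lowers clamped health, stores the damage and impact normal, and prints debug text, including "dead" at zero; the AnyDamage handler is disabled.
; HealthSystem calls Ragdoll at zero health, which stops movement, disables capsule collision, simulates mesh physics and sets Isdead.
; Nothing in this file calls HealthSystem, so radial damage alone does not trigger the ragdoll here.
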(event Game|Damage|EventRadialDamage
  (params (DamageReceived :type Float%20%28single-precision%29) (DamageType :type Damage%20Type%20Object%20Reference) (Origin :type Vector :default "0, 0, 0") (HitInfo :type Hit%20Result%20Structure%20%28by%20ref%29) (InstigatedBy :type Controller%20Object%20Reference) (DamageCauser :type Actor%20Object%20Reference))
  (Variables|Default|Setdamage%20recieved DamageReceived)
  (Variables|Default|SetImpact%20Normal%20origin (.ImpactNormal (Collision|BreakHitResult HitInfo)))
  (bind _output_get (Variables|Default|Sethealth (Math|Float|Clamp(Float) (- (Variables|Default|Gethealth) (Variables|Default|Getdamage%20recieved)) 0.0 (Variables|Default|GetmaxHealth))))
  (Development|PrintString (Utilities|String|ToString(Float) _output_get))
  (if (<= (Variables|Default|Gethealth) 0.0)
    (Development|PrintString "dead")))

(event Game|Damage|EventAnyDamage
  (params (Damage :type Float%20%28single-precision%29) (DamageType :type Damage%20Type%20Object%20Reference) (InstigatedBy :type Controller%20Object%20Reference) (DamageCauser :type Actor%20Object%20Reference))
  ;[1 0 0] disabled
)

(fn ConstructionScript)

(fn HealthSystem
  (if (<= (Variables|Default|Gethealth) 0.0)
    (CallFunction|Ragdoll)))

(fn Ragdoll
  (bind _mesh (Variables|Character|GetMesh))
  (Utilities|FlowControl|Sequence
    (:then_0
      (Pawn|Components|CharacterMovement|SetMovementMode (Variables|Character|GetCharacterMovement) "MOVE_None" 0))
    (:then_1
      (Collision|SetCollisionEnabled (Variables|Collision|GetCapsuleComponent) "NoCollision")
      (Collision|SetCollisionObjectType _mesh "ECC_PhysicsBody")
      (Collision|SetCollisionEnabled _mesh "PhysicsOnly")
      (Physics|SetSimulatePhysics _mesh true))
    (:then_2
      (Variables|Default|Setisdead true))))