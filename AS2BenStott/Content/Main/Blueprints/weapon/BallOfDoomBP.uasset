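; BallOfDoomBP is a damaging weapon ball that expires after two seconds if it hits no character.
; Overlapping a characterBP applies BaseDamage, then destroys the ball; other actors are ignored.
; If that character's PlayerHealth is at or below zero, it ragdolls, loses movement and input, and takes a damage-scaled impulse against the hit normal, with blood and splat sound at the impact point.
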(event OnComponentBeginOverlap(collision)
  (params (OverlappedComponent :type Primitive%20Component%20Object%20Reference) (OtherActor :type Actor%20Object%20Reference) (OtherComp :type Primitive%20Component%20Object%20Reference) (OtherBodyIndex :type Integer) (bFromSweep :type Boolean) (SweepResult :type Hit%20Result%20Structure%20%28by%20ref%29))
  (bind (_bblockinghit _binitialoverlap _time _distance _location _impactpoint _normal) (Collision|BreakHitResult SweepResult))
  (bind _base_damage (Variables|Default|GetBase%20Damage))
  (bind _ascharacter_bp (Utilities|Casting|CastTocharacterBP OtherActor))
  (Utilities|FlowControl|Sequence
    (:then_0
      (Game|Damage|ApplyDamage _ascharacter_bp (Variables|Default|GetBase%20Damage) 0 0)
      (Variables|Default|SetimpactOrigin _normal)
      (if (<= (Variables|/Game/Main/Blueprints/characters/characterBP.characterBP_C|GetplayerHealth _ascharacter_bp) 0.0)
        (Physics|SetSimulatePhysics (Variables|/Script/Engine.Character|GetMesh _ascharacter_bp) true)
        (Collision|SetCollisionProfileName (Variables|/Script/Engine.Character|GetMesh _ascharacter_bp) "RagDoll" true :!class /Script/Engine.PrimitiveComponent)
        (Pawn|Components|CharacterMovement|DisableMovement (Variables|/Script/Engine.Character|GetCharacterMovement _ascharacter_bp))
        (Input|DisableInput _ascharacter_bp (Game|GetPlayerController 0))
        (Physics|AddImpulseatLocation (Variables|/Script/Engine.Character|GetMesh _ascharacter_bp) (Math|Vector|MakeVector (* _base_damage (* (.x (Variables|Default|GetimpactOrigin)) -5e+02)) (* _base_damage (* (.y (Variables|Default|GetimpactOrigin)) -5e+02)) (* _base_damage (* (.z (Variables|Default|GetimpactOrigin)) -5e+02))) _impactpoint "None")
        (Effects|SpawnEmitteratLocation "/Game/Main/Imported/Particles/Blood/P_Blood_Splat_Cone.P_Blood_Splat_Cone" _impactpoint "0, 0, 0" "0.400000,0.400000,0.400000")
        (Audio|PlaySoundatLocation "/Game/Main/Imported/sounds/splattt-6295.splattt-6295" _impactpoint "0, 0, 0" 1.0 1.0 0.0 0 0 0 0)))
    (:then_1
      (Actor|DestroyActor))))

(event EventBeginPlay
  (Actor|SetLifeSpan 2.0))

(fn ConstructionScript)